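; Player pawn that moves by physics torque on its mesh and restarts the current level when it takes any damage.
; Forward/back and right/left input axes apply torque scaled by AccelMultiplier as an acceleration change, so mass is ignored.
; BeginPlay fades the camera in, while damage triggers a DoOnce-guarded RestartLevel that fades out, waits, and reopens the level by name.
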(event `self.ReceiveBeginPlay`
  ;[1 1 1] Fade in on begin play
  (`PlayerCameraManager.StartCameraFade` :`self` (`GameplayStatics.GetPlayerCameraManager` 0) :`FromAlpha` 1.0 :`Duration` 3.0))

(event `self.ReceiveAnyDamage`
  (params (Damage :type "Float (single-precision)") (DamageType :type "DamageType Object Reference") (InstigatedBy :type "Controller Object Reference") (DamageCauser :type "Actor Object Reference"))
  (`self.RestartLevel`))

(event `InputAxis|Move Forwards/Backwards`
  (params (AxisValue :type "Float (single-precision)"))
  ;[1 1 1] Movement
  (`PrimitiveComponent.AddTorqueInRadians` (`self.Mesh`) (`KismetMathLibrary.MakeVector` 0.0 (* AxisValue (`self.accelMultiplier`))) "None" true))

(event `InputAxis|Move Right/Left`
  (params (AxisValue :type "Float (single-precision)"))
  ;[1 1 1] Movement
  (`PrimitiveComponent.AddTorqueInRadians` (`self.Mesh`) (`KismetMathLibrary.MakeVector` (* AxisValue (`self.accelMultiplier`))) "None" true))

(fn `UserConstructionScript`)