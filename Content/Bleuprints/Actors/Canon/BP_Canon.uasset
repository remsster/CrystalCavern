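; BP_Canon is a cannon actor that automatically fires projectiles on a repeating cycle from BeginPlay.
; After a FireRate delay, it spawns a BP_Projectile at the ProjectileSpawnPoint's location and rotation, scaled by ProjectileScale.
; A timeline then animates the barrel along its relative Y axis, and its Cannon Fired event track loops back to the delay for the next shot.
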(event `self.ReceiveBeginPlay`
  (`KismetSystemLibrary.Delay` (`self.FireRate`) :!label _label)
  (`self.SpawnProjectile`)
  (bind (_direction _cannonbarrellocation) (`Timeline|CannonFireTimeline` :!via `PlayFromStart`)
    (:`Update`
      (`self.MoveCannonBarrel` _cannonbarrellocation))
    (:`Cannon Fired`
      (goto _label))))

(fn `MoveCannonBarrel`
  (params (Cannon_Barrel_Y_Location :type "Float (double-precision)"))
  (`SceneComponent.K2_SetRelativeLocation` (`self.Cannon_Barrel`) (`KismetMathLibrary.MakeVector` 0.0 Cannon_Barrel_Y_Location) false false))

(fn `SpawnProjectile`
  (bind _projectile_spawn_point (`self.Projectile_spawn_point`))
  (`|SpawnActorFromClass` "/Game/Bleuprints/Actors/Projectiles/BP_Projectile.BP_Projectile_C" (`KismetMathLibrary.MakeTransform` (`SceneComponent.K2_GetComponentLocation` _projectile_spawn_point) (`SceneComponent.K2_GetComponentRotation` _projectile_spawn_point) (`KismetMathLibrary.Conv_DoubleToVector` (`self.ProjectileScale`))) "Undefined" "OverrideRootScale" null null))

(fn `UserConstructionScript`)